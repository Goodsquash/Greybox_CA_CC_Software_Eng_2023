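; Moving board actor that travels along the spline of a Spline_Path_BP actor, starting on BeginPlay.
; MoveObject plays a timeline at a rate of 1 / TimeToCompleteInSeconds, mapping its track onto spline distance to set location and rotation.
; Location is sampled in world space but rotation in local space.
; BeginPlay looks up the path actor but sets SplineREF to None, so the found actor never reaches the movement logic.
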(event Custom|Move%20Object
  (bind _spline_ref (Variables|Default|GetSpline%20REF))
  (bind _spline (Variables|Components|GetSpline _spline_ref))
  (Components|Timeline|SetPlayRate (Variables|Default|GetMove%20Object%20T) (/ 1.0 (Variables|Default|GetTime%20to%20complete%20%28in%20seconds%29)))
  (bind _newtrack_0 (Timeline|Move%20Object%20T Play)
    (:Update
      (Transformation|SetActorTransform (Math|Transform|MakeTransform (Spline|GetLocationatDistanceAlongSpline _spline (Math|Float|Lerp 0.0 (Spline|GetSplineLength (Variables|Components|GetSpline (.Spline%20REF (Variables|Default|GetSpline%20REF)))) _newtrack_0) "World") (Spline|GetRotationatDistanceAlongSpline _spline (Math|Float|Lerp 0.0 (Spline|GetSplineLength (Variables|Components|GetSpline (.Spline%20REF (Variables|Default|GetSpline%20REF)))) _newtrack_0) "Local") "1.000000,1.000000,1.000000")))))

(event EventBeginPlay
  (bind _returnvalue (Actor|GetActorOfClass "/Game/Blueprints/Spline_Path_BP.Spline_Path_BP_C"))
  (Variables|Default|SetSpline%20REF 0 _returnvalue)
  (CallFunction|MoveObject))

(fn ConstructionScript)