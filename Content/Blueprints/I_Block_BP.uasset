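; I_Block_BP is a moving hazard block that knocks down and hurts the third-person player character on contact.
; On BeginPlay it picks the start or end point component as its target, then each tick slides toward it at constant speed without sweeping.
; The target is never switched afterward, so it travels one way.
; Box overlap ragdolls the character, applies damage and plays a punch sound.
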(event OnComponentBeginOverlap(Box)
  (params (OverlappedComponent :type Primitive%20Component%20Object%20Reference) (OtherActor :type Actor%20Object%20Reference) (OtherComp :type Primitive%20Component%20Object%20Reference) (OtherBodyIndex :type Integer) (bFromSweep :type Boolean) (SweepResult :type Hit%20Result%20Structure%20%28by%20ref%29))
  (bind _asbp_third_person_character (Utilities|Casting|CastToBP_ThirdPersonCharacter OtherActor))
  (Default|Ragdoll _asbp_third_person_character)
  (Game|Damage|ApplyDamage _asbp_third_person_character 15.0 0 0)
  (Audio|PlaySound2D "/Game/Music_and_Sounds/punch-boxing-02wav-14897_Cue.punch-boxing-02wav-14897_Cue" 1.0 1.0 0.0 0 0))

(event EventBeginPlay
  (Variables|Default|SetCurrent%20Location (Transformation|GetActorLocation))
  (Variables|Default|SetStart%20Point%20Location (Transformation|GetWorldLocation (Variables|Default|GetStart%20Point)))
  (Variables|Default|SetEnd%20Point%20Location (Transformation|GetWorldLocation (Variables|Default|GetEnd%20Point)))
  (if (Variables|Default|GetMove%20to%20Start%20Point)
    (Variables|Default|SetTarget%20Location (Variables|Default|GetStart%20Point%20Location))
    (else
      (Variables|Default|SetTarget%20Location (Variables|Default|GetEnd%20Point%20Location)))))

(event EventTick
  (params (DeltaSeconds :type Float%20%28single-precision%29))
  (Variables|Default|SetFrame%20Time DeltaSeconds)
  (bind _output_get (Variables|Default|SetCurrent%20Location (Math|Interpolation|VInterptoConstant (Variables|Default|GetCurrent%20Location) (Variables|Default|GetTarget%20Location) (Variables|Default|GetFrame%20Time) (Variables|Default|GetMovement%20Speed))))
  (Transformation|SetActorLocation _output_get false false))

(fn ConstructionScript)