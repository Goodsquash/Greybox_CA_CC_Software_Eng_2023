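; Pickup actor, named as a health pickup, that bobs up and down and disappears when the player character touches it.
; From BeginPlay, an endless latent loop eases the Invinc component between the Bottom and Top markers' relative locations, pausing briefly at each end.
; Overlap on Invinc destroys the actor if the other actor is BP_ThirdPersonCharacter; this graph applies no health or invincibility effect.
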(event OnComponentBeginOverlap(Invinc)
  (params (OverlappedComponent :type Primitive%20Component%20Object%20Reference) (OtherActor :type Actor%20Object%20Reference) (OtherComp :type Primitive%20Component%20Object%20Reference) (OtherBodyIndex :type Integer) (bFromSweep :type Boolean) (SweepResult :type Hit%20Result%20Structure%20%28by%20ref%29))
  (Utilities|Casting|CastToBP_ThirdPersonCharacter OtherActor)
  (Actor|DestroyActor))

(event EventBeginPlay
  (bind _invinc (Variables|Default|GetInvinc))
  ;[1 1 1] Up Down Movement
  (Components|MoveComponentTo _invinc (Variables|/Script/Engine.SceneComponent|GetRelativeLocation (Variables|Default|GetBottom)) "0, 0, 0" true true 2.0 false :!label _label)
  (Utilities|FlowControl|Delay 0.1)
  (Components|MoveComponentTo _invinc (Variables|/Script/Engine.SceneComponent|GetRelativeLocation (Variables|Default|GetTop)) "0, 0, 0" true true 2.0 false)
  (Utilities|FlowControl|Delay 0.1)
  (goto _label))

(fn ConstructionScript)