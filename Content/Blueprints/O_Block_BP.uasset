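; O_Block_BP is a moving hazard block that damages the third-person character when it touches its box.
; BeginPlay picks the start or end point component's world location as a fixed target from a flag, and Tick moves the block there at constant speed without sweeping or reversing.
; Overlap deals three timed damage hits a second apart, with an explosion on the first and fire on the following two.
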(event OnComponentBeginOverlap(Box)
  (params (OverlappedComponent :type Primitive%20Component%20Object%20Reference) (OtherActor :type Actor%20Object%20Reference) (OtherComp :type Primitive%20Component%20Object%20Reference) (OtherBodyIndex :type Integer) (bFromSweep :type Boolean) (SweepResult :type Hit%20Result%20Structure%20%28by%20ref%29))
  (bind _asbp_third_person_character (Utilities|Casting|CastToBP_ThirdPersonCharacter OtherActor))
  (Game|Damage|ApplyDamage _asbp_third_person_character 5.0 0 0)
  (Effects|SpawnEmitteratLocation "/Game/StarterContent/Particles/P_Explosion.P_Explosion" (Transformation|GetActorLocation _asbp_third_person_character) "0, 0, 0" "2.000000,2.000000,2.000000")
  (Utilities|FlowControl|Delay 1.0)
  (Game|Damage|ApplyDamage _asbp_third_person_character 5.0 0 0)
  (Effects|SpawnEmitteratLocation "/Game/StarterContent/Particles/P_Fire.P_Fire" (Transformation|GetActorLocation _asbp_third_person_character) "0, 0, 0" "2.000000,2.000000,2.000000")
  (Utilities|FlowControl|Delay 1.0)
  (Game|Damage|ApplyDamage _asbp_third_person_character 5.0 0 0)
  (Effects|SpawnEmitteratLocation "/Game/StarterContent/Particles/P_Fire.P_Fire" (Transformation|GetActorLocation _asbp_third_person_character) "0, 0, 0" "2.000000,2.000000,2.000000"))

(event EventBeginPlay
  (Variables|Default|SetCurrent%20Location (Transformation|GetActorLocation))
  (Variables|Default|SetStart%20Point%20Location (Transformation|GetWorldLocation (Variables|Default|GetStart%20Point)))
  (Variables|Default|SetEnd%20Point%20Location (Transformation|GetWorldLocation (Variables|Default|GetEnd%20Point)))
  (if (Variables|Default|GetMove%20to%20Start%20Point)
    (Variables|Default|SetTarget%20Location (Variables|Default|GetStart%20Point%20Location))
    (else
      (Variables|Default|SetTarget%20Location (Variables|Default|GetEnd%20Point%20Location)))))

(event EventTick
  (params (DeltaSeconds :type Float%20%28single-precision%29))
  (Variables|Default|SetFrame%20Time DeltaSeconds)
  (bind _output_get (Variables|Default|SetCurrent%20Location (Math|Interpolation|VInterptoConstant (Variables|Default|GetCurrent%20Location) (Variables|Default|GetTarget%20Location) (Variables|Default|GetFrame%20Time) (Variables|Default|GetMovement%20Speed))))
  (Transformation|SetActorLocation _output_get false false))

(fn ConstructionScript)